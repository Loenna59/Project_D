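; BP_PlayerCharacter is the player character Blueprint, with a P key toggle between first-person and third-person views.
; Each press flips IsFirstPerson, then changes the CameraBoom's arm length and relative height to move the view.
; First person uses a negative arm length and hides the mesh from the Neck bone down its hierarchy, and third person restores it.
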(event `Key|P`
  (params (Key :type "Key Structure"))
  (bind _cameraboom (`self.CameraBoom`))
  (bind _mesh (`self.Mesh`))
  (:`Pressed`
    (bind _output_get (set `self.bIsFirstPerson` (not (`self.bIsFirstPerson`))))
    (if _output_get
      (set `SpringArmComponent.TargetArmLength` -20.0 _cameraboom)
      (`SceneComponent.K2_SetRelativeLocation` _cameraboom (0.0 0.0 85.0) false false)
      (`SkinnedMeshComponent.HideBoneByName` _mesh "Neck" "PBO_None")
      (else
        (set `SpringArmComponent.TargetArmLength` 200.0 _cameraboom)
        (`SceneComponent.K2_SetRelativeLocation` _cameraboom (0.0 0.0 138.492264) false false)
        (`SkinnedMeshComponent.UnHideBoneByName` _mesh "Neck")))))

(fn `UserConstructionScript`)