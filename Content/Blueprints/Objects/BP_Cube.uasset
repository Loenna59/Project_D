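; BP_Cube is a physics cube that launches upward at BeginPlay, then drifts and tumbles under continuous procedural forces.
; BeginPlay enables physics simulation and adds an upward velocity impulse to the Cube component.
; Each Tick applies a smoothly varying force from time-sampled Perlin noise, using a different frequency per axis.
; Tick also adds a new random torque as a mass-independent acceleration, producing erratic spin.
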(event `self.ReceiveBeginPlay`
  (bind _cube (`self.Cube`))
  (`PrimitiveComponent.SetSimulatePhysics` _cube true)
  (`PrimitiveComponent.SetPhysicsLinearVelocity` _cube (0.0 0.0 1000.0) true "None"))

(event `self.ReceiveTick`
  (params (DeltaSeconds :type "Float (single-precision)"))
  (bind _returnvalue (`GameplayStatics.GetTimeSeconds`))
  (bind _returnvalue_2 (`KismetMathLibrary.RandomFloatInRange` -500.0 500.0))
  (`PrimitiveComponent.AddForce` (`self.Cube`) (* (`KismetMathLibrary.MakeVector` (`KismetMathLibrary.PerlinNoise1D` (* _returnvalue 0.5)) (`KismetMathLibrary.PerlinNoise1D` (* _returnvalue 0.3)) (`KismetMathLibrary.PerlinNoise1D` (* _returnvalue 0.7))) 1000.0) "None" false)
  (`PrimitiveComponent.AddTorqueInRadians` (`self.Cube`) (`KismetMathLibrary.MakeVector` _returnvalue_2 _returnvalue_2 _returnvalue_2) "None" true))

(fn `UserConstructionScript`)